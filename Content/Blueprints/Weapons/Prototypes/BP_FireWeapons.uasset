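; Prototype firearm weapon that extends a parent UseWeapon with hitscan damage, ammo readouts and reloading.
; Without a projectile class, UseWeapon line-traces from the player camera along the owner's forward vector, applying point damage; with one, it only returns success.
; A failed use triggers Reload on an empty magazine with reserves left.
; IsReloading's RepNotify starts an authority-side timer, whose completion sets magazine ammo to the computed reload amount and deducts reserves.
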(event Custom|Debug_GetFireTrace
  (params (Start :type Vector) (End :type Vector) (Hit :type Vector))
  (Rendering|Debug|DrawDebugLine Start End "(R=0.729167,G=0.599753,B=0.000000,A=1.000000)" 5.0 2.0)
  (Rendering|Debug|DrawDebugSphere Hit 2e+01 8 "(R=1.000000,G=0.000000,B=0.107245,A=1.000000)" 5.0 2.0))

(fn ConstructionScript
  (|CallParentFunction))

(fn UseWeapon
  (bind _used (|CallParentFunction))
  (if _used
    (Development|PrintString (Utilities|String|Append (Utilities|String|ToString(Integer) (Variables|Default|GetCurrentAmmo)) "|" (Utilities|String|ToString(Integer) (Variables|Default|GetTotalAmmo))) true true "(R=0.000000,G=1.000000,B=0.077879,A=1.000000)" 1.0 "1")
    (if (Utilities|IsValidClass (Variables|Default|GetFireProjectile))
      (return true)
      (else
        ;[1 1 1] Fired
        (bind _hit (CallFunction|GetFireTrace))
        (Game|Damage|ApplyPointDamage (.HitActor (Collision|BreakHitResult _hit)) (Variables|Default|GetDamage) (Math|Vector|GetUnitDirection(Vector) (.TraceEnd (Collision|BreakHitResult _hit)) (.TraceStart (Collision|BreakHitResult _hit))) _hit (Game|GetInstigatorController) self)
        (return true)))
    (else
      (Development|PrintString "Reloading!" true true "(R=1.000000,G=0.876469,B=0.014936,A=1.000000)" 1.0 "1")
      (if (and (<= (Variables|Default|GetCurrentAmmo) 0) (> (Variables|Default|GetTotalAmmo) 0))
        (CallFunction|Reload)
        (return false)
        (else
          (return false))))))

(fn GetFireTrace
  (bind _asbp_player_character (Utilities|Casting|CastToBP_PlayerCharacter (Game|GetInstigator)))
  (bind _outhit (Collision|LineTraceForObjects (Transformation|GetWorldLocation (Variables|/Game/Blueprints/Player/Prototypes/BP_PlayerCharacter.BP_PlayerCharacter_C|GetCamera _asbp_player_character)) (+ (Transformation|GetWorldLocation (Variables|/Game/Blueprints/Player/Prototypes/BP_PlayerCharacter.BP_PlayerCharacter_C|GetCamera _asbp_player_character)) (* (Transformation|GetActorForwardVector (Components|GetOwner)) 10000)) (Utilities|Array|MakeArray "ObjectTypeQuery1" "ObjectTypeQuery2" "ObjectTypeQuery3") false (Utilities|Array|MakeArray self (Game|GetInstigator)) "None"))
  (CallFunction|DebugGetFireTrace (.TraceStart (Collision|BreakHitResult _outhit)) (.TraceEnd (Collision|BreakHitResult _outhit)) (.Location (Collision|BreakHitResult _outhit)))
  (return _outhit))

(fn Reload
  (if (not (Variables|Default|GetIsReloading))
    (Variables|Default|SetIsReloading true)))

(fn OnRepIsReloading
  (Networking|SwitchHasAuthority
    (:Authority
      (if (Variables|Default|GetIsReloading)
        (if (Math|Boolean|ANDBoolean (< (Variables|Default|GetCurrentAmmo) (.CurrentAmmo (Utilities|GetClassDefaults (Utilities|GetClass self)))) (> (Variables|Default|GetTotalAmmo) 0) (not (Utilities|Time|IsValidTimerHandle (LocalVariables|GetTimer))))
          (Variables|Default|SetAmmoToReload (Math|Integer|Min(Integer) (- (.CurrentAmmo (Utilities|GetClassDefaults (Utilities|GetClass self))) (Variables|Default|GetCurrentAmmo)) (Variables|Default|GetTotalAmmo)))
          (bind _returnvalue (Utilities|Time|SetTimerbyFunctionName 0 "ReloadFinished" (Variables|Default|GetReloadTime)))
          (LocalVariables|SetTimer _returnvalue)
          (else
            (Variables|Default|SetIsReloading false)))))))

(fn ReloadFinished
  (Variables|Default|SetCurrentAmmo (Variables|Default|GetAmmoToReload))
  (Variables|Default|SetTotalAmmo (- (Variables|Default|GetTotalAmmo) (Variables|Default|GetAmmoToReload)))
  (Variables|Default|SetIsReloading false))