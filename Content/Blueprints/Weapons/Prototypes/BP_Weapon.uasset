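; BP_Weapon is a prototype weapon Blueprint that handles trigger state, ammo use and fire-rate limiting, with no projectile, hit or effect logic.
; UseWeapon checks for ammo and cooldown, spends one round, starts a UseRate timer and returns whether the shot succeeded.
; When the timer expires, StopRateDelay clears the cooldown and calls UseWeapon again if AutoFire is on and the trigger is still held.
; ReleaseWeaponTrigger clears the fire state, ending that loop.
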(fn ConstructionScript)

(fn UseWeapon
  (Variables|Default|SetInFireState true)
  (if (CallFunction|AbletoUseWeapon)
    (Math|Integer|DecrementInt (Variables|Default|GetCurrentAmmo)
      (:%20%20
        (Utilities|Time|SetTimerbyFunctionName 0 "StopRateDelay" (Variables|Default|GetUseRate))
        (Variables|Default|SetUseFreezedByRate true)
        (return true)))
    (else
      (Variables|Default|SetInFireState false)
      (return false))))

(fn AbletoUseWeapon
  (return (and (> (Variables|Default|GetCurrentAmmo) 0) (not (Variables|Default|GetUseFreezedByRate)))))

(fn StopRateDelay
  (Variables|Default|SetUseFreezedByRate false)
  (if (and (Variables|Default|GetAutoFire) (Variables|Default|GetInFireState))
    (CallFunction|UseWeapon)))

(fn ReleaseWeaponTrigger
  (Variables|Default|SetInFireState false))