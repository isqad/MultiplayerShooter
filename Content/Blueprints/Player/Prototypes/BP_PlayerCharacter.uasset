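; Prototype player character Blueprint with mouse look, directional movement and networked weapon firing.
; Primary action press and release call server events that use the current weapon or release its trigger through BPWeaponManager.
; On possession, the authority creates and selects an autorifle through the same manager.
; GetVisibleSkeletalMesh returns the Arms mesh when locally controlled and the body Mesh otherwise.
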(event Custom|ServerFire
  ;[1 1 1] Run on Server
  (Default|UseWeapon (Variables|/Game/Blueprints/Components/Prototypes/Player/BP_WeaponManager.BP_WeaponManager_C|GetCurrentWeapon (Variables|Default|GetBP_WeaponManager))))

(event Custom|ServerFireStop
  ;[1 1 1] Run on Server
  (Default|ReleaseWeaponTrigger (Variables|/Game/Blueprints/Components/Prototypes/Player/BP_WeaponManager.BP_WeaponManager_C|GetCurrentWeapon (Variables|Default|GetBP_WeaponManager))))

(event EventPossessed
  (params (NewController :type Controller%20Object%20Reference))
  (bind _bp_weaponmanager (Variables|Default|GetBP_WeaponManager))
  (Networking|SwitchHasAuthority
    (:Authority
      (bind _weapon (Default|CreateWeapon _bp_weaponmanager "/Game/Blueprints/Weapons/Prototypes/BP_Weapon_Autoriffle.BP_Weapon_Autoriffle_C"))
      (Default|SelectWeapon _bp_weaponmanager _weapon))))

(event Input|ActionEvents|InputActionPrimaryAction
  (params (Key :type Key%20Structure :default "None"))
  ;[1 1 1] Run on client
  (:Pressed
    (CallFunction|ServerFire))
  (:Released
    (CallFunction|ServerFireStop)))

(event Input|AxisEvents|InputAxisMoveForward
  (params (AxisValue :type Float%20%28single-precision%29))
  (Pawn|Input|AddMovementInput (Transformation|GetActorForwardVector) AxisValue false))

(event Input|AxisEvents|InputAxisLookUpMouse
  (params (AxisValue :type Float%20%28single-precision%29))
  (Pawn|Input|AddControllerPitchInput AxisValue))

(event Input|AxisEvents|InputAxisTurnRightMouse
  (params (AxisValue :type Float%20%28single-precision%29))
  (Pawn|Input|AddControllerYawInput AxisValue))

(event Input|AxisEvents|InputAxisMoveRight
  (params (AxisValue :type Float%20%28single-precision%29))
  (Pawn|Input|AddMovementInput (Transformation|GetActorRightVector) AxisValue false))

(fn ConstructionScript)

(fn GetVisibleSkeletalMesh
  (if (Pawn|IsLocallyControlled)
    (return (Variables|Default|GetArms))
    (else
      (return (Variables|Character|GetMesh)))))