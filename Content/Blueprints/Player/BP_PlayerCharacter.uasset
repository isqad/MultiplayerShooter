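; BP_PlayerCharacter is the networked player character, with mouse look and movement relative to the actor's forward and right vectors.
; On BeginPlay, only the authority creates an autorifle through BPWeaponManager and selects it.
; GetVisibleSkeletalMesh returns the Arms mesh for the locally controlled player and the body Mesh otherwise, separating first-person from third-person visuals.
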(event EventBeginPlay
  (bind _bp_weaponmanager (Variables|Default|GetBP_WeaponManager))
  (Networking|SwitchHasAuthority
    (:Authority
      (bind _weapon (Default|CreateWeapon _bp_weaponmanager "/Game/Blueprints/Weapons/BP_Weapon_Autoriffle.BP_Weapon_Autoriffle_C"))
      (Default|SelectWeapon _bp_weaponmanager _weapon))))

(event Input|AxisEvents|InputAxisMoveForward
  (params (AxisValue :type Float%20%28single-precision%29))
  (Pawn|Input|AddMovementInput (Transformation|GetActorForwardVector) AxisValue false))

(event Input|AxisEvents|InputAxisLookUpMouse
  (params (AxisValue :type Float%20%28single-precision%29))
  (Pawn|Input|AddControllerPitchInput AxisValue))

(event Input|AxisEvents|InputAxisTurnRightMouse
  (params (AxisValue :type Float%20%28single-precision%29))
  (Pawn|Input|AddControllerYawInput AxisValue))

(event Input|AxisEvents|InputAxisMoveRight
  (params (AxisValue :type Float%20%28single-precision%29))
  (Pawn|Input|AddMovementInput (Transformation|GetActorRightVector) AxisValue false))

(fn ConstructionScript)

(fn GetVisibleSkeletalMesh
  (if (Pawn|IsLocallyControlled)
    (return (Variables|Default|GetArms))
    (else
      (return (Variables|Character|GetMesh)))))