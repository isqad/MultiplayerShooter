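; Player weapon manager component that spawns, stores and equips the owning BP_PlayerCharacter's weapons.
; CreateWeapon runs server-only, spawning a BP_Weapon, filing it by WeaponType into main, secondary, special, grenade or melee storage and attaching it to the character.
; SelectWeapon sets CurrentWeapon, whose RepNotify attaches it to the visible skeletal mesh's GripPoint socket on clients only.
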(event EventBeginPlay
  (bind _asbp_player_character (Utilities|Casting|CastToBP_PlayerCharacter (Components|GetOwner)))
  (Variables|Default|SetCharacter _asbp_player_character))

(fn CreateWeapon
  (params (Class :type Actor%20Class%20Reference))
  (bind _character (Variables|Default|GetCharacter))
  (if (Networking|IsServer)
    (bind _returnvalue (Game|SpawnActorfromClass Class (Math|Transform|MakeTransform "0, 0, 0" "0, 0, 0" "1.000000,1.000000,1.000000") "AlwaysSpawn" (Pawn|GetController _character) _character))
    (bind _asbp_weapon (Utilities|Casting|CastToBP_Weapon _returnvalue))
    (bind _output_get (LocalVariables|SetL_Weapon _asbp_weapon))
    (switch Utilities|FlowControl|Switch|SwitchonE_WeaponType (Variables|/Game/Blueprints/Weapons/Prototypes/BP_Weapon.BP_Weapon_C|GetWeaponType _output_get)
      (:NewEnumerator0
        (Variables|Default|SetMainWeapon (LocalVariables|GetL_Weapon)))
      (:NewEnumerator1
        (Variables|Default|SetSecondaryWeapon (LocalVariables|GetL_Weapon)))
      (:NewEnumerator2
        (Utilities|Array|Add (Variables|Default|GetSpecialWeapons) (LocalVariables|GetL_Weapon)))
      (:NewEnumerator3
        (Utilities|Array|Add (Variables|Default|GetGrenades) (LocalVariables|GetL_Weapon)))
      (:NewEnumerator4
        (Variables|Default|SetMeleeWeapon (LocalVariables|GetL_Weapon))))
    (Transformation|AttachActorToActor (LocalVariables|GetL_Weapon) (Variables|Default|GetCharacter) "None" "SnapToTarget" "SnapToTarget" "KeepRelative" true)
    (return (LocalVariables|GetL_Weapon))))

(fn SelectWeapon
  (params (Weapon :type BP%20Weapon%20Object%20Reference))
  (Variables|Default|SetCurrentWeapon Weapon))

(fn OnRepCurrentWeapon
  (if (not (Networking|IsServer))
    (Transformation|AttachComponentToComponent (Variables|Default|GetCurrentWeapon) (Default|GetVisibleSkeletalMesh (Variables|Default|GetCharacter)) "GripPoint" "KeepRelative" "KeepRelative" "KeepRelative" true)))