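; Prototype health component for BP_PlayerCharacter that handles damage, armor and death.
; On the server, BeginPlay binds to the owner's AnyDamage event and feeds each hit into ApplyDamage.
; Math-expression nodes scale damage by armor and wear armor down, and depleted health sets IsDead.
; The IsDead RepNotify disables movement and ragdolls the mesh, with debug prints throughout.
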(event Custom|OnPlayerTakeAnyDamage
  (params (DamagedActor :type Actor%20Object%20Reference) (Damage :type Float%20%28single-precision%29) (DamageType :type Damage%20Type%20Object%20Reference) (InstigatedBy :type Controller%20Object%20Reference) (DamageCauser :type Actor%20Object%20Reference))
  (Development|PrintString (Utilities|String|Append "Damage: " (Utilities|String|ToString(Float) Damage)) true true "(R=0.263333,G=1.000000,B=0.347283,A=1.000000)")
  (CallFunction|ApplyDamage Damage))

(event EventBeginPlay
  (Networking|SwitchHasAuthority
    (:Authority
      (bind _asbp_player_character (Utilities|Casting|CastToBP_PlayerCharacter (Components|GetOwner)))
      (bind _output_get (Variables|Default|SetCharacter _asbp_player_character))
      (EventDispatchers|AssignOnTakeAnyDamage _output_get (EventDispatchers|CreateEvent :!event Custom|OnPlayerTakeAnyDamage)))))

(fn ApplyDamage
  (params (Damage :type Float%20%28double-precision%29))
  (LocalVariables|SetLDamage (|(Damage*(1-({8B82AC12-40AF-4DC7-E0BB-9F907184555A}/200))) Damage))
  (Variables|Default|SetHealth (- (Variables|Default|GetHealth) (LocalVariables|GetLDamage)))
  (Variables|Default|SetArmor (|(max(({8B82AC12-40AF-4DC7-E0BB-9F907184555A}-(2*Damage)),0)) (LocalVariables|GetLDamage)))
  (Development|PrintString (Utilities|String|ToString(Float) (LocalVariables|GetLDamage)) true true "(R=1.000000,G=0.961748,B=0.000000,A=1.000000)")
  (if (<= (Variables|Default|GetHealth) 0.0)
    (Variables|Default|SetIsDead true)))

(fn OnRepIsDead
  (bind _character (Variables|Default|GetCharacter))
  (Pawn|Components|CharacterMovement|DisableMovement (Variables|/Script/Engine.Character|GetCharacterMovement _character))
  (Physics|SetSimulatePhysics (Variables|/Script/Engine.Character|GetMesh _character) true)
  (Development|PrintString "Character go away" true true "(R=0.893636,G=1.000000,B=0.868238,A=1.000000)"))